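; AI controller for BP_Runner that simulates a player's alternating left and right power inputs.
; On possession it caches the runner and prints its name.
; BeginPlay starts a looping timer with one random interval between the min and max input delay, apparently driving SimulateInput, whose FlipFlop alternates SimulatePowerLeft and SimulatePowerRight on the runner.
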(event Custom|SimulateInput
  (Utilities|FlowControl|FlipFlop
    (:A
      (Default|SimulatePowerLeft (Variables|Default|GetOwningRunner)))
    (:B
      (Default|SimulatePowerRight (Variables|Default|GetOwningRunner)))))

(event EventBeginPlay
  (Utilities|Time|SetTimerbyEvent (EventDispatchers|CreateEvent :!event Custom|SimulateInput) (Math|Random|RandomFloatinRange (Variables|Default|GetMinInputDelay) (Variables|Default|GetMaxInputDelay)) true))

(event EventPossess
  (params (PossessedPawn :type Pawn%20Object%20Reference))
  (bind _asbp_runner (Utilities|Casting|CastToBP_Runner PossessedPawn))
  (bind _output_get (Variables|Default|SetOwningRunner _asbp_runner))
  (Development|PrintString (Utilities|GetDisplayName _output_get)))

(fn ConstructionScript)